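; Dial_BP is a trigger volume that plays a scripted dialogue as floating text when the player pawn overlaps its box.
; It steps through the Dialogues array, moving a single text render above each line's AI speaker and setting its sentence.
; Each line's display time scales with its character count, clamped to a minimum and maximum.
; Nothing blocks re-triggering or clears the last line when the sequence ends.
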(event `self.Box.OnComponentBeginOverlap`
  (params (OverlappedComponent :type "PrimitiveComponent Object Reference") (OtherActor :type "Actor Object Reference") (OtherComp :type "PrimitiveComponent Object Reference") (OtherBodyIndex :type Integer) (bFromSweep :type Boolean) (SweepResult :type "HitResult Structure (by ref)"))
  (cast `/Game/Blueprints/PlayerPawn` OtherActor)
  (`self.StartDialogue`))

(event `StartDialogue`
  (bind _returnvalue (`KismetArrayLibrary.Array_Length` (`self.Dialogues`)))
  (bind _item (`KismetArrayLibrary.Array_Get` (`self.Dialogues`) (`self.IndexDial`)))
  (if (> _returnvalue 0)
    (set `self.IndexDial` 0)
    (if (< (`self.IndexDial`) _returnvalue) :!label _label
      (`self.UpdateText` _item)
      (bind _delay (`self.SentenceDelay` _item))
      (`KismetSystemLibrary.Delay` _delay)
      (`/Engine/EditorBlueprintResources/StandardMacros.IncrementInt` (`self.IndexDial`)
        (:`  `
          (goto _label))))))

(fn `SentenceDelay`
  (params (Sentence :type "/Game/Blueprints/Mine/Dial_struct Structure"))
  (returns (Delay :type "Float (double-precision)"))
  (return (`KismetMathLibrary.FClamp` (* (`KismetStringLibrary.Len` (`KismetTextLibrary.Conv_TextToString` (`.Sentence_5_E40C7ADE46004E2FFB7F279A1FDE30DF` (break `/Game/Blueprints/Mine/Dial_struct` Sentence)))) 0.2) 1.0 10.0)))

(fn `UpdateText`
  (params (Sentence :type "/Game/Blueprints/Mine/Dial_struct Structure"))
  (bind (_ai _sentence) (break `/Game/Blueprints/Mine/Dial_struct` Sentence))
  (bind _textrender (`self.TextRender`))
  (`TextRenderComponent.K2_SetText` _textrender _sentence)
  (`SceneComponent.K2_SetWorldLocation` _textrender (+ (`self.K2_GetActorLocation` _ai) (0.0 0.0 150.0)) false false))

(fn `UserConstructionScript`)