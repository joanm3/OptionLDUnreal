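; Dialogue actor that plays a sequence of sentences as floating text above the AI actor assigned to each line.
; StartDialogue shows the Text and Arrow components, then a latent Delay loop steps through the Dialogues array, moving the text over each sentence's actor.
; Each line's display time scales with its character count.
; After the last sentence, it hides the components and calls CallEndDialogEvent.
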(event `DialogueStart`
  (bind _indexdial (`self.IndexDial`))
  (bind _returnvalue (`KismetArrayLibrary.Array_Length` (`self.Dialogues`)))
  (bind _item (`KismetArrayLibrary.Array_Get` (`self.Dialogues`) _indexdial))
  (if (!= _returnvalue 0)
    (set `self.IndexDial` 0)
    (if (< _indexdial _returnvalue) :!label _label
      (`self.SetText` _item)
      (`KismetSystemLibrary.Delay` (`self.GetSentenceDelay` _item))
      (`/Engine/EditorBlueprintResources/StandardMacros.IncrementInt` (`self.IndexDial`)
        (:`  `
          (goto _label)))
      (else
        (`self.ShowDialogue` false)
        (`self.EndDialogEvent`)))))

(fn `GetSentenceDelay`
  (params (Sentence :type "/Game/Blueprints/Dialogue_Sentence_Struct Structure"))
  (returns (Delay :type "Float (double-precision)"))
  (return (* (`KismetStringLibrary.Len` (`.Sentence_5_BE64A1C6420632608746C49C36770058` (break `/Game/Blueprints/Dialogue_Sentence_Struct` Sentence))) 0.2)))

(fn `SetText`
  (params (Sentence :type "/Game/Blueprints/Dialogue_Sentence_Struct Structure"))
  (bind (_ai _sentence) (break `/Game/Blueprints/Dialogue_Sentence_Struct` Sentence))
  (bind _text (`self.text`))
  (`TextRenderComponent.K2_SetText` _text (`KismetTextLibrary.Conv_StringToText` _sentence))
  (`SceneComponent.K2_SetWorldLocation` _text (+ (`self.K2_GetActorLocation` _ai) (0.0 0.0 140.0)) false false))

(fn `ShowDialogue`
  (params (bShow :type Boolean))
  (if bShow
    (`SceneComponent.SetHiddenInGame` (`self.Arrow`) false false)
    (`SceneComponent.SetHiddenInGame` (`self.text`) false false)
    (else
      (`SceneComponent.SetHiddenInGame` (`self.text`) true false)
      (`SceneComponent.SetHiddenInGame` (`self.Arrow`) true false))))

(fn `StartDialogue`
  (`self.ShowDialogue` true)
  (`self.DialogueStart`))

(fn `UserConstructionScript`)